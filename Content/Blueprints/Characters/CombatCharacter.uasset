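; CombatCharacter is a combat actor that automatically attacks its Enemy at an interval set by AttackSpeed.
; Tick drives a Delay loop that subtracts damage until the enemy's health reaches zero, then sets this character's own IsDefeated flag.
; SetDamage rolls between minimum and maximum damage, both scaled by the main attribute.
; Hits on a CombatCharacter_Player reduce health stored in the GameInstance, then copy it to that character.
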(event EventBeginPlay
  (bind _asmy_hero_game_instance (Utilities|Casting|CastToMyHeroGameInstance (Game|GetGameInstance)))
  (Variables|Default|SetgameInstance _asmy_hero_game_instance))

(event EventTick
  (params (DeltaSeconds :type Float%20%28single-precision%29))
  (bind _gameinstance (Variables|Default|GetgameInstance))
  (bind _enemy (Variables|Default|Getenemy))
  (Utilities|FlowControl|Delay (Variables|Default|GetattackSpeed) :!label _label)
  (bind _newparam (CallFunction|SetDamage))
  (Variables|Default|Setdamage _newparam)
  (if (== (Utilities|GetClass (Variables|Default|Getenemy)) "/Game/Blueprints/Characters/CombatCharacter_Player.CombatCharacter_Player_C")
    (bind _output_get (Variables|/Game/Blueprints/MyHeroGameInstance.MyHeroGameInstance_C|SetcurrentHealth _gameinstance (- (Variables|/Game/Blueprints/MyHeroGameInstance.MyHeroGameInstance_C|GetcurrentHealth _gameinstance) (Variables|Default|Getdamage))))
    (Variables|CombatCharacter_C|SetcurrentCombatHealth (Variables|Default|Getenemy) _output_get)
    (else
      (Variables|CombatCharacter_C|SetcurrentCombatHealth _enemy (- (Variables|CombatCharacter_C|GetcurrentCombatHealth _enemy) (Variables|Default|Getdamage)))))
  (if (<= (Variables|CombatCharacter_C|GetcurrentCombatHealth (Variables|Default|Getenemy)) 0)
    (Variables|CombatCharacter_C|SetcurrentCombatHealth (Variables|Default|Getenemy) 0)
    (Variables|Default|SetisDefeated true)
    (else
      (goto _label))))

(fn ConstructionScript)

(fn SetDamage
  (switch Utilities|FlowControl|Switch|SwitchonmainStat (Variables|Default|GetmainAtt)
    (:NewEnumerator0
      (LocalVariables|Setmultiplier (Variables|Default|Getagility)))
    (:NewEnumerator1
      (LocalVariables|Setmultiplier (Variables|Default|Getintelligence)))
    (:NewEnumerator2
      (LocalVariables|Setmultiplier (Variables|Default|Getstrength))))
  (LocalVariables|SettempMaxDamage (* (Variables|Default|GetmaxDamage) (LocalVariables|Getmultiplier)))
  (LocalVariables|SettempMinDamage (* (Variables|Default|GetminDamage) (LocalVariables|Getmultiplier)))
  (return (Math|Random|RandomIntegerinRange (LocalVariables|GettempMinDamage) (LocalVariables|GettempMaxDamage))))