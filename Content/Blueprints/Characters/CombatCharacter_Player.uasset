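; CombatCharacter_Player is the player's combat character, which loads its attributes from the game instance when play begins.
; On BeginPlay it calls PlayerGetAtts, which casts the game instance to MyHeroGameInstance and stores the reference.
; It then copies Strength, Intelligence, Agility, and current health and energy into its own variables.
; Values flow one way, with no write-back to the game instance in this Blueprint.
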(event EventBeginPlay
  (|CallParentFunction)
  (CallFunction|PlayerGetAtts))

(event Collision|EventActorBeginOverlap
  (params (OtherActor :type Actor%20Object%20Reference))
  (|CallParentFunction OtherActor) ; This node is disabled and will not be called.\nDrag off pins to build functionality.
)

(event EventTick
  (params (DeltaSeconds :type Float%20%28single-precision%29))
  (|CallParentFunction DeltaSeconds) ; This node is disabled and will not be called.\nDrag off pins to build functionality.
)

(fn ConstructionScript
  (|CallParentFunction))

(fn PlayerGetAtts
  (bind _asmy_hero_game_instance (Utilities|Casting|CastToMyHeroGameInstance (Game|GetGameInstance)))
  (Variables|Default|SetgameInstance _asmy_hero_game_instance)
  (Utilities|FlowControl|Sequence
    (:then_0
      (Variables|Default|Setstrength (Variables|/Game/Blueprints/MyHeroGameInstance.MyHeroGameInstance_C|Getstrength (Variables|Default|GetgameInstance))))
    (:then_1
      (Variables|Default|Setintelligence (Variables|/Game/Blueprints/MyHeroGameInstance.MyHeroGameInstance_C|Getintelligence (Variables|Default|GetgameInstance))))
    (:then_2
      (Variables|Default|Setagility (Variables|/Game/Blueprints/MyHeroGameInstance.MyHeroGameInstance_C|Getagility (Variables|Default|GetgameInstance))))
    (:then_3
      (Variables|Default|Sethealth (Variables|/Game/Blueprints/MyHeroGameInstance.MyHeroGameInstance_C|GetcurrentHealth (Variables|Default|GetgameInstance))))
    (:then_4
      (Variables|Default|Setenergy (Variables|/Game/Blueprints/MyHeroGameInstance.MyHeroGameInstance_C|GetcurrentEnergy (Variables|Default|GetgameInstance))))))