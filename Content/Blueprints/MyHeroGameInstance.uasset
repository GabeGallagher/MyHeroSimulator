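; MyHeroGameInstance is a Game Instance Blueprint, by its name, that holds the hero's energy, health and minutes counters.
; Three setter functions apply relative changes: SetEnergy and SetTime add the amount, while SetHealth subtracts it, so a positive value acts as damage.
; None of the functions clamps the result or notifies other objects.
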(fn SetEnergy
  (params (amt :type Integer))
  (Variables|Default|SetcurrentEnergy (+ (Variables|Default|GetcurrentEnergy) amt)))

(fn SetTime
  (params (amt :type Integer))
  (Variables|Default|Setminutes (+ (Variables|Default|Getminutes) amt)))

(fn SetHealth
  (params (amt :type Integer))
  (Variables|Default|SetcurrentHealth (- (Variables|Default|GetcurrentHealth) amt)))