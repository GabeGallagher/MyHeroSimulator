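; Clickable workout station that trains one hero attribute (Agility, Strength or Intelligence, chosen by Type) at a cost in time and energy.
; Clicking registers it as the GameInstance's ClickedActor and starts a Delay loop on WaitTime.
; Each pass calls SetTime with WorkTime, then, while still the clicked actor, adds StatModifier to the attribute, applies EnergyTax and repeats.
; Attribute, time and energy changes all go through MyHeroGameInstance.
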(event EventBeginPlay)

(event Collision|EventActorBeginOverlap
  (params (OtherActor :type Actor%20Object%20Reference)))

(event EventTick
  (params (DeltaSeconds :type Float%20%28single-precision%29)))

(event MouseInput|EventActorOnClicked
  (params (ButtonPressed :type Key%20Structure))
  (bind _asmy_hero_game_instance (Utilities|Casting|CastToMyHeroGameInstance (Game|GetGameInstance))
    (:then
      (bind _output_get (Variables|Default|SetgameInstance _asmy_hero_game_instance))
      (Variables|/Game/Blueprints/MyHeroGameInstance.MyHeroGameInstance_C|SetclickedActor _output_get self)
      (Utilities|FlowControl|Delay (Variables|Default|GetwaitTime) :!label _label)
      (Default|SetTime (Variables|Default|GetgameInstance) (Variables|Default|GetworkTime))
      (bind _out (CallFunction|GetAttributebyType))
      (if (== (Variables|/Game/Blueprints/MyHeroGameInstance.MyHeroGameInstance_C|GetclickedActor (Variables|Default|GetgameInstance)) self)
        (CallFunction|SetAttributebyType (+ _out (Variables|Default|GetstatModifier)))
        (Default|SetEnergy (Variables|Default|GetgameInstance) (* (Variables|Default|GetenergyTax) -1))
        (goto _label)))
    (:CastFailed
      (Development|PrintString (Utilities|String|Append (Utilities|GetDisplayName self) " failed to cast to My Hero Game Instance") true true "(R=0.000000,G=0.660000,B=1.000000,A=1.000000)" 1e+01))))

(fn ConstructionScript)

(fn GetAttributebyType
  (switch Utilities|FlowControl|Switch|SwitchonStationType (Variables|Default|Gettype)
    (:NewEnumerator0
      (return (Variables|/Game/Blueprints/MyHeroGameInstance.MyHeroGameInstance_C|Getagility (Variables|Default|GetgameInstance))))
    (:NewEnumerator1
      (return (Variables|/Game/Blueprints/MyHeroGameInstance.MyHeroGameInstance_C|Getstrength (Variables|Default|GetgameInstance))))
    (:NewEnumerator2
      (return (Variables|/Game/Blueprints/MyHeroGameInstance.MyHeroGameInstance_C|Getintelligence (Variables|Default|GetgameInstance))))))

(fn SetAttributebyType
  (params (newAmount :type Integer))
  (Variables|Default|SetnewAmount newAmount)
  (switch Utilities|FlowControl|Switch|SwitchonStationType (Variables|Default|Gettype)
    (:NewEnumerator0
      (Variables|/Game/Blueprints/MyHeroGameInstance.MyHeroGameInstance_C|Setagility (Variables|Default|GetgameInstance) (Variables|Default|GetnewAmount)))
    (:NewEnumerator1
      (Variables|/Game/Blueprints/MyHeroGameInstance.MyHeroGameInstance_C|Setstrength (Variables|Default|GetgameInstance) (Variables|Default|GetnewAmount)))
    (:NewEnumerator2
      (Variables|/Game/Blueprints/MyHeroGameInstance.MyHeroGameInstance_C|Setintelligence (Variables|Default|GetgameInstance) (Variables|Default|GetnewAmount)))))