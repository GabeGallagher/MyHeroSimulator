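; StoreCounter is a clickable store counter actor that opens the store menu when clicked.
; On click it runs the parent handler, creates a StoreMenu widget, and casts the GameInstance's ClickedActor to StoreCounter.
; It passes that counter to the widget before adding it to the viewport, so the inventory is accessible while the menu builds.
; A failed cast only prints an error.
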(event EventBeginPlay)

(event MouseInput|EventActorOnClicked
  (params (ButtonPressed :type Key%20Structure))
  (|CallParentFunction "")
  (bind _returnvalue (UserInterface|CreateWidget "/Game/UI/Menus/StoreMenu.StoreMenu_C"))
  (Variables|Default|SetstoreMenu _returnvalue)
  ;[1 1 1] set menu store object reference so that the inventory is accessible when the store menu is built
  (bind _asstore_counter (Utilities|Casting|CastToStoreCounter (Variables|/Game/Blueprints/MyHeroGameInstance.MyHeroGameInstance_C|GetclickedActor (Variables|Default|GetgameInstance)))
    (:then
      (Variables|/Game/UI/Menus/StoreMenu.StoreMenu_C|SetstoreCounterObject (Variables|Default|GetstoreMenu) _asstore_counter)
      (UserInterface|Viewport|AddtoViewport (Variables|Default|GetstoreMenu) 0))
    (:CastFailed
      (Development|PrintString "Cast to store counter failed"))))

(fn ConstructionScript)